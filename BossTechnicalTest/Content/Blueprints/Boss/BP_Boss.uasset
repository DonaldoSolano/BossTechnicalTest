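; Troll boss character with three montage attacks, a health bar widget updated each tick, and ragdoll death.
; Montage notifies fire sphere traces from the hammer, or mouth for the vomit attack, applying damage and camera shake on hit.
; AnyDamage lowers health; at zero it notifies BP_AI_Boss, stops movement, plays a death montage, then ragdolls.
; SelectRandomDeathMontage always yields the first montage, as RandomInteger(1) returns zero and both branches read index 0.
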(event EventAttackB
  (bind _hammer (Variables|Default|GetHammer))
  (bind _returnvalue (Transformation|GetWorldLocation _hammer))
  ;[0.15 0.15 0.15 0.5] Play anim montage AttackB when attack function is called and apply damage by sweeping a sphere trace from the Troll's hammer
  (if (not (Variables|Attack|GetbIsAttacking))
    (Animation|Montage|PlayMontage (Variables|Character|GetMesh) "/Game/Characters/Boss/Troll/Montages/ExoGame_Troll_Attack_Overhead_Montage.ExoGame_Troll_Attack_Overhead_Montage"
      (:then
        (Variables|Attack|SetbIsAttacking true))
      (:OnCompleted
        (Variables|Attack|SetbIsAttacking false))
      (:OnNotifyBegin
        (Camera|PlayWorldCameraShake "/Game/Blueprints/Boss/BP_Hammer_ground_hit_CameraShake.BP_Hammer_ground_hit_CameraShake_C" (Transformation|GetWorldLocation (Variables|Default|GetHammer)) 0.0 4e+03)
        (bind (_outhit _returnvalue_2) (Collision|SphereTraceForObjects _returnvalue (+ _returnvalue (* (Math|Vector|GetForwardVector (Transformation|GetWorldRotation _hammer)) 1.0)) 1.7e+02 (Utilities|Array|MakeArray "ObjectTypeQuery3") false 0 "ForDuration" true "(R=1.000000,G=0.000000,B=0.000000,A=1.000000)" "(R=0.000000,G=1.000000,B=0.000000,A=1.000000)" 2.0))
        (if _returnvalue_2
          (Game|Damage|ApplyDamage (.HitActor (Collision|BreakHitResult _outhit)) (Variables|Attack|GetAttackBDamage) 0 0)
          (Camera|PlayWorldCameraShake "/Game/Blueprints/Boss/BP_CameraShake.BP_CameraShake_C" (Transformation|GetActorLocation) 0.0 4e+03))))))

(event EventAttackC
  (bind _mouthdirection (Variables|Default|GetMouthDirection))
  (bind _returnvalue (Transformation|GetWorldLocation _mouthdirection))
  ;[0.15 0.15 0.15 0.5] Play anim montage AttackC when attack function is called and apply damage by sweeping a sphere trace from the Troll's hammer
  (if (not (Variables|Attack|GetbIsAttacking))
    (Animation|Montage|PlayMontage (Variables|Character|GetMesh) "/Game/Characters/Boss/Troll/Montages/ExoGame_Troll_Attack_Vomit_Montage.ExoGame_Troll_Attack_Vomit_Montage"
      (:then
        (Variables|Attack|SetbIsAttacking true))
      (:OnCompleted
        (Variables|Attack|SetbIsAttacking false))
      (:OnNotifyBegin
        (bind (_outhit _returnvalue_2) (Collision|SphereTraceForObjects _returnvalue (+ _returnvalue (* (Math|Vector|GetForwardVector (Transformation|GetWorldRotation _mouthdirection)) 3e+02)) 1.7e+02 (Utilities|Array|MakeArray "ObjectTypeQuery3") false 0 "ForDuration" true "(R=1.000000,G=0.000000,B=0.000000,A=1.000000)" "(R=0.000000,G=1.000000,B=0.000000,A=1.000000)" 2.0))
        (if _returnvalue_2
          (Game|Damage|ApplyDamage (.HitActor (Collision|BreakHitResult _outhit)) (Variables|Attack|GetAttackCDamage) 0 0)
          (Camera|PlayWorldCameraShake "/Game/Blueprints/Boss/BP_CameraShake.BP_CameraShake_C" (Transformation|GetActorLocation) 0.0 4e+03))))))

(event EventAttack
  (bind _hammer (Variables|Default|GetHammer))
  (bind _returnvalue (Transformation|GetWorldLocation _hammer))
  ;[0.15 0.15 0.15 0.5] Play anim montage when attack function is called and apply damage by sweeping a sphere trace from the Troll's hammer
  (if (not (Variables|Attack|GetbIsAttacking))
    (Animation|Montage|PlayMontage (Variables|Character|GetMesh) "/Game/Characters/Boss/Troll/Montages/ExoGame_Troll_Attack_Montage.ExoGame_Troll_Attack_Montage"
      (:then
        (Variables|Attack|SetbIsAttacking true))
      (:OnCompleted
        (Variables|Attack|SetbIsAttacking false))
      (:OnNotifyBegin
        (bind (_outhit _returnvalue_2) (Collision|SphereTraceForObjects _returnvalue (+ _returnvalue (* (Math|Vector|GetForwardVector (Transformation|GetWorldRotation _hammer)) 1.0)) 1.7e+02 (Utilities|Array|MakeArray "ObjectTypeQuery3") false 0 "ForDuration" true "(R=1.000000,G=0.000000,B=0.000000,A=1.000000)" "(R=0.000000,G=1.000000,B=0.000000,A=1.000000)" 2.0))
        (if _returnvalue_2
          (Game|Damage|ApplyDamage (.HitActor (Collision|BreakHitResult _outhit)) (Variables|Attack|GetAttackADamage) 0 0)
          (Camera|PlayWorldCameraShake "/Game/Blueprints/Boss/BP_CameraShake.BP_CameraShake_C" (Transformation|GetActorLocation) 0.0 4e+03))))))

(event EventBeginPlay
  ;[0.15 0.15 0.15 0.5] Create boss health bar widget at the beginning of the gameplay
  (bind _returnvalue (UserInterface|CreateWidget "/Game/Blueprints/Boss/WBP_Boss_health.WBP_Boss_health_C"))
  (UserInterface|Viewport|AddtoViewport _returnvalue 0)
  (Variables|Health|SetWBP_Boss_health _returnvalue))

(event EventTick
  (params (DeltaSeconds :type Float%20%28single-precision%29))
  ;[0.15 0.15 0.15 0.5] Update widget progress bar percentage per frame
  (Progress|SetPercent (Variables|/Game/Blueprints/Boss/WBP_Boss_health.WBP_Boss_health_C|GetHealthBar (Variables|Health|GetWBP_Boss_health)) (/ (Variables|Health|GetHealth) 1e+02)))

(event Game|Damage|EventAnyDamage
  (params (Damage :type Float%20%28single-precision%29) (DamageType :type Damage%20Type%20Object%20Reference) (InstigatedBy :type Controller%20Object%20Reference) (DamageCauser :type Actor%20Object%20Reference))
  ;[0.15 0.15 0.15 0.5] Reduce life based on damage and disable character movement, activate ragdoll on death and detach AI controller
  (Variables|Health|SetHealth (- (Variables|Health|GetHealth) Damage))
  (Default|CallOnHealthChange (Variables|Health|GetHealth))
  (if (<= (Variables|Health|GetHealth) 0.0)
    (bind _asbp_ai_boss (Utilities|Casting|CastToBP_AI_Boss (Pawn|GetController)))
    (Default|BossDeath _asbp_ai_boss)
    (Pawn|Components|CharacterMovement|DisableMovement (Variables|Character|GetCharacterMovement))
    (bind _animmontage (CallFunction|SelectRandomDeathMontage))
    (Animation|Montage|PlayMontage (Variables|Character|GetMesh) _animmontage
      (:OnCompleted
        (Physics|SetSimulatePhysics (Variables|Character|GetMesh) true)
        (Collision|SetCollisionEnabled (Variables|Collision|GetCapsuleComponent) "NoCollision")
        (Default|CallOnDeath)))))

(fn ConstructionScript)

(fn SelectRandomDeathMontage
  (bind _animmontages (Variables|Death|GetAnimMontages))
  ;[0.15 0.15 0.15 0.5] Select a random animation montage out of an array of two montages
  (switch int (Math|Random|RandomInteger 1)
    (:0
      (if (Utilities|Array|IsValidIndex _animmontages)
        (bind _output_get (Variables|Death|SetRandomDeathMontage (Utilities|Array|Get(acopy) _animmontages)))
        (return _output_get)
        (else
          (Development|PrintString "Not valid index 0"))))
    (:1
      (if (Utilities|Array|IsValidIndex _animmontages 1)
        (Variables|Death|SetRandomDeathMontage (Utilities|Array|Get(acopy) _animmontages))
        (return _output_get)
        (else
          (Development|PrintString "Not valid index 1"))))))