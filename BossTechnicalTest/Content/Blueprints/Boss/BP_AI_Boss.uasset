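; AI controller for the boss that runs the BT_Boss behavior tree and feeds its blackboard.
; Pawn sensing sets the target-seen flag and stores the player's location for rotate-to-face, and SeePlayer can also set the flag.
; Boss health changes are mirrored to the blackboard through an event binding.
; Player death clears the flag and stops sensing, while BossDeath detaches the controlled pawn from the controller.
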(event OnSeePawn(PawnSensing)
  (params (Pawn :type Pawn%20Object%20Reference))
  ;[0.15 0.15 0.15 0.5] bIsSeeingTarget = true if sensing the player
  (AI|Components|Blackboard|SetValueasBool (AI|GetBlackboard 0) (Utilities|Name|MakeLiteralName "bIsSeeingTarget") true)
  ;[0.15 0.15 0.15 0.5] Update the rotate to face BB entry Vector Value key of the behavior tree with the player character position
  (AI|Components|Blackboard|SetValueasVector (AI|GetBlackboard 0) (Utilities|Name|MakeLiteralName "VectorKey") (Transformation|GetActorLocation (Game|GetPlayerCharacter 0))))

(event Custom|BossDeath
  ;[0.15 0.15 0.15 0.5] Call detach when Boss dies
  (Class|Pawn|DetachfromControllerPendingDestroy (Pawn|GetControlledPawn)))

(event Custom|StopSensing
  ;[0.15 0.15 0.15 0.5] Set bIsSeeingTarget to false and disable the pawn sensing component updates after player dies
  (Class|PawnSensingComponent|SetSensingUpdatesEnabled (Variables|Default|GetPawnSensing) false)
  (AI|Components|Blackboard|SetValueasBool (AI|GetBlackboard 0) (Utilities|Name|MakeLiteralName "bIsSeeingTarget") false))

(event Custom|HealthChange
  (params (Health :type Float%20%28double-precision%29))
  ;[0.15 0.15 0.15 0.5] Run behavior tree on gameplay start
  (AI|Components|Blackboard|SetValueasFloat (AI|GetBlackboard 0) (Utilities|Name|MakeLiteralName "Health") Health))

(event Custom|SeePlayer
  ;[0.15 0.15 0.15 0.5] Event that sets bIsSeeingPlayer black board key to true
  (AI|Components|Blackboard|SetValueasBool (AI|GetBlackboard 0) (Utilities|Name|MakeLiteralName "bIsSeeingTarget") true))

(event EventBeginPlay
  ;[0.15 0.15 0.15 0.5] Run behavior tree on gameplay start
  (Utilities|FlowControl|Sequence
    (:then_0
      (AI|RunBehaviorTree "/Game/Blueprints/Boss/BT_Boss.BT_Boss")
      (bind _asbp_third_person_character (Utilities|Casting|CastToBP_ThirdPersonCharacter (Game|GetPlayerCharacter 0)))
      (EventDispatchers|BindEventtoOnDeath _asbp_third_person_character (delegate Custom|StopSensing)))
    (:then_1
      (bind _asbp_boss (Utilities|Casting|CastToBP_Boss (Pawn|GetControlledPawn)))
      (EventDispatchers|BindEventtoOnHealthChange _asbp_boss (delegate Custom|HealthChange)))))

(fn ConstructionScript)